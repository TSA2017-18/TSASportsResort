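; BP_MiniGolf_Hole is the mini-golf hole that detects when a player's PWN_MiniGolf pawn has finished.
; An overlap on the player collision waits briefly, then marks the pawn Done only if it still overlaps the hole.
; A separate toggle volume switches off collision on the game state's landscape actor while a pawn enters, and restores it when a pawn leaves.
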(event OnComponentBeginOverlap(PlayeCollision)
  (params (OverlappedComponent :type Primitive%20Component%20Object%20Reference) (OtherActor :type Actor%20Object%20Reference) (OtherComp :type Primitive%20Component%20Object%20Reference) (OtherBodyIndex :type Integer) (bFromSweep :type Boolean) (SweepResult :type Hit%20Result%20Structure%20%28by%20ref%29))
  (Utilities|FlowControl|Delay 0.3)
  (if (Collision|IsOverlappingActor OtherActor self :!class /Script/Engine.Actor)
    (bind _aspwn_mini_golf (Utilities|Casting|CastToPWN_MiniGolf OtherActor))
    (Variables|/Game/Pawns/PWN_MiniGolf.PWN_MiniGolf_C|SetDone _aspwn_mini_golf true)))

(event OnComponentEndOverlap(TerrainCollisionToggle)
  (params (OverlappedComponent :type Primitive%20Component%20Object%20Reference) (OtherActor :type Actor%20Object%20Reference) (OtherComp :type Primitive%20Component%20Object%20Reference) (OtherBodyIndex :type Integer))
  (Utilities|Casting|CastToPWN_MiniGolf OtherActor)
  (bind _asgs_mini_golf_multiplayer (Utilities|Casting|CastToGS_MiniGolf_Multiplayer (Game|GetGameState)))
  (Collision|SetActorEnableCollision (Variables|/Game/GameStates/GS_MiniGolf_Multiplayer.GS_MiniGolf_Multiplayer_C|GetLandscapeActor _asgs_mini_golf_multiplayer) true)
  (bind _output_get (Variables|Default|SetCollision "QueryAndPhysics"))
  (|SetBy-RefVar (.CollisionEnabled (Utilities|Struct|BreakBodyInstance (Variables|/Script/Landscape.LandscapeProxy|GetBodyInstance (Variables|/Game/GameStates/GS_MiniGolf_Multiplayer.GS_MiniGolf_Multiplayer_C|GetLandscapeActor _asgs_mini_golf_multiplayer)))) _output_get))

(event OnComponentBeginOverlap(TerrainCollisionToggle)
  (params (OverlappedComponent :type Primitive%20Component%20Object%20Reference) (OtherActor :type Actor%20Object%20Reference) (OtherComp :type Primitive%20Component%20Object%20Reference) (OtherBodyIndex :type Integer) (bFromSweep :type Boolean) (SweepResult :type Hit%20Result%20Structure%20%28by%20ref%29))
  (Utilities|Casting|CastToPWN_MiniGolf OtherActor)
  (bind _asgs_mini_golf_multiplayer (Utilities|Casting|CastToGS_MiniGolf_Multiplayer (Game|GetGameState)))
  (Collision|SetActorEnableCollision (Variables|/Game/GameStates/GS_MiniGolf_Multiplayer.GS_MiniGolf_Multiplayer_C|GetLandscapeActor _asgs_mini_golf_multiplayer) false)
  (bind _output_get (Variables|Default|SetCollision "NoCollision"))
  (|SetBy-RefVar (.CollisionEnabled (Utilities|Struct|BreakBodyInstance (Variables|/Script/Landscape.LandscapeProxy|GetBodyInstance (Variables|/Game/GameStates/GS_MiniGolf_Multiplayer.GS_MiniGolf_Multiplayer_C|GetLandscapeActor _asgs_mini_golf_multiplayer)))) _output_get))

(event EventBeginPlay)

(event Collision|EventActorBeginOverlap
  (params (OtherActor :type Actor%20Object%20Reference)))

(event EventTick
  (params (DeltaSeconds :type Float%20%28single-precision%29)))

(fn ConstructionScript)