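; Spline generator Blueprint that lays a chosen static mesh along its spline during construction.
; The construction script stores the point count, resizes SplineDataArray to match, then calls BuildSplineElement over the point indices.
; Each call adds a spline mesh component fitted to the local locations and tangents of the current and next point, with a modulo wrap linking last back to first.
; SplineDataArray is not read when building segments.
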(event EventBeginPlay)

(event Collision|EventActorBeginOverlap
  (params (OtherActor :type Actor%20Object%20Reference)))

(event EventTick
  (params (DeltaSeconds :type Float%20%28single-precision%29)))

(fn ConstructionScript
  (bind _spline_data_array (Variables|Default|GetSpline%20Data%20Array))
  (Utilities|FlowControl|Sequence
    (:then_0
      (|Storenumberofsplinepoints))
    (:then_1
      (Math|Integer|CompareInt (Utilities|Array|Length _spline_data_array) (Variables|Default|GetNum%20spline%20pts) :!label _label
        (:>
          (Utilities|Array|RemoveIndex _spline_data_array (Utilities|Array|LastIndex _spline_data_array))
          (goto _label))
        (:<
          (Utilities|Array|Add :TargetArray _spline_data_array)
          (goto _label))))
    (:then_2
      (for _index (range 0 (Variables|Default|GetNum%20spline%20pts))
        (CallFunction|BuildSplineElement _index (Variables|Default|GetSplineMesh))))
    (:then_3)))

(fn BuildSplineElement
  (params (LoopIndex :type Integer) (Spline%20Mesh%20Element%20 :type Static%20Mesh%20Object%20Reference))
  (bind _output_get (LocalVariables|SetL_CurrentLoopIndex LoopIndex))
  (LocalVariables|SetL_NextLoopIndex (Math|Integer|%(Integer) (+ _output_get 1) (Variables|Default|GetNum%20spline%20pts)))
  (LocalVariables|SetL_SplineElementMesh Spline%20Mesh%20Element%20)
  (Utilities|FlowControl|Sequence
    (:then_0
      (LocalVariables|SetL_StartLoacation (.Location (Spline|GetLocationandTangentatSplinePoint (Variables|Default|GetSpline) (LocalVariables|GetL_CurrentLoopIndex) "Local")))
      (LocalVariables|SetL_StartTangent (.Tangent (Spline|GetLocationandTangentatSplinePoint (Variables|Default|GetSpline) (LocalVariables|GetL_CurrentLoopIndex) "Local")))
      (LocalVariables|SetL_EndLocation (.Location (Spline|GetLocationandTangentatSplinePoint (Variables|Default|GetSpline) (LocalVariables|GetL_NextLoopIndex) "Local")))
      (LocalVariables|SetL_EndTangent (.Tangent (Spline|GetLocationandTangentatSplinePoint (Variables|Default|GetSpline) (LocalVariables|GetL_NextLoopIndex) "Local"))))
    (:then_1
      (bind _returnvalue (AddComponent|AddSplineMeshComponent false))
      (bind _output_get_2 (LocalVariables|SetL_CurrentSplineMesh _returnvalue))
      (Components|StaticMesh|SetStaticMesh _output_get_2 (LocalVariables|GetL_SplineElementMesh))
      (SplineMesh|SetStartandEnd (LocalVariables|GetL_CurrentSplineMesh) (LocalVariables|GetL_StartLoacation) (LocalVariables|GetL_StartTangent) (LocalVariables|GetL_EndLocation) (LocalVariables|GetL_EndTangent) true :!class /Script/Engine.SplineMeshComponent))))